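; BP_Scoreboard is a card game scoreboard that declares the player or AI the winner as soon as play begins.
; On BeginPlay it prints the value of every BP_Card tagged "Card", then fires OnConditionsMet to print the result from CountCards.
; CountCards overwrites player points with each card's value and zeroes enemy points, so the last card alone decides the winner.
; The cards' player and AI possession flags are unused.
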(event `self.ReceiveBeginPlay`
  (bind _outactors (`GameplayStatics.GetAllActorsOfClassWithTag` "/Script/Engine.Actor" "Card"))
  (for _array_element _outactors
    (bind _asbp_card (cast `/Game/Dynamic/BP_Card` _array_element))
    (`KismetSystemLibrary.PrintText` (`KismetTextLibrary.Conv_IntToText` (`/Game/Dynamic/BP_Card.CardValue` _asbp_card))))
  (`self.Event On Conditions Met`))

(event `Event On Conditions Met`
  (bind _playerwin (`self.CountCards` null))
  (if _playerwin
    (`KismetSystemLibrary.PrintText` "Player wins")
    (else
      (`KismetSystemLibrary.PrintText` "AI wins"))))

(fn `CountCards`
  (params (Cards :type "Actor Object Reference"))
  (returns (PlayerWin :type Boolean))
  (locals (PlayerPoints :type Integer) (EnemyPoints :type Integer))
  ;[0.01042 0.01042 0.01042] Sets points based on the cards on the table
  (bind _outactors (`GameplayStatics.GetAllActorsOfClassWithTag` "/Script/Engine.Actor" "Card"))
  (for _array_element _outactors
    (bind _asbp_card (cast `/Game/Dynamic/BP_Card` _array_element))
    (set `local.PlayerPoints` (`/Game/Dynamic/BP_Card.CardValue` _asbp_card))
    (set `local.EnemyPoints` 0))
  (if (> (`local.PlayerPoints`) (`local.EnemyPoints`))
    (return true)
    (else
      (return false))))

(fn `UserConstructionScript`)