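; Game mode for a card game in which a player and an AI alternately draw cards from a BP_DeckManager deck.
; BeginPlay resets the deck and loops both turns until each side has drawn three cards or either draws a Death card.
; Turns add non-Death card values to the BP_Scoreboard game state, which calculates points after the loop.
; Only the player's draw spawns a BP_Card actor to show the card.
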(event `self.ReceiveBeginPlay`
  (bind _outactors (`GameplayStatics.GetAllActorsOfClass` "/Game/Dynamic/CardGame/Blueprints/BP_DeckManager.BP_DeckManager_C"))
  (set `self.DeckManagerRef` (`|GetArrayItem` _outactors))
  (`/Game/Dynamic/CardGame/Blueprints/BP_DeckManager.ResetDeck` (`self.DeckManagerRef`))
  (set `self.CurrentTurn` "NewEnumerator0")
  (for _ (range 11)
    ;[1 1 1] Loops between each turns
    (if (or (and (>= (`self.PlayerCardsDrawn`) 3) (>= (`self.AI CardsDrawn`) 3)) (or (`self.PlayerDrewDeath`) (`self.AI DrewDeath`)))
      (break)
      (else
        (`self.PlayerTurnLogic`)
        (`self.AI TurnLogic`))))
  ;[1 1 1] Calculate points afterwards
  (bind _asbp_scoreboard (cast `/Game/Dynamic/CardGame/Blueprints/BP_Scoreboard` (`GameplayStatics.GetGameState`)))
  (`/Game/Dynamic/CardGame/Blueprints/BP_Scoreboard.CalculatePoints` _asbp_scoreboard))

(fn `AI TurnLogic`
  (returns (`AI Points` :type Integer))
  (bind _ai_cardsdrawn (`self.AI CardsDrawn`))
  (set `self.CurrentTurn` "NewEnumerator1")
  (`KismetSystemLibrary.PrintString` (`KismetStringLibrary.Concat_StrStr` "Player is drawing card. Cards drawn: " (`KismetStringLibrary.Conv_IntToString` _ai_cardsdrawn)))
  (`/Engine/EditorBlueprintResources/StandardMacros.IncrementInt` _ai_cardsdrawn
    (:`  `
      (bind _carddrawn (`/Game/Dynamic/CardGame/Blueprints/BP_DeckManager.DrawCard` (`self.DeckManagerRef`)))
      (bind _output_get (set `self.AICard` _carddrawn))
      (bind (_cardvalue _isdeathcard_) (break `/Game/Dynamic/CardGame/S_Card` _output_get))
      (if _isdeathcard_
        (`KismetSystemLibrary.PrintString` "ai drew death")
        (set `self.AI DrewDeath` true)
        (else
          (`KismetSystemLibrary.PrintString` (`KismetStringLibrary.Conv_IntToString` _cardvalue))
          (bind _asbp_scoreboard (cast `/Game/Dynamic/CardGame/Blueprints/BP_Scoreboard` (`GameplayStatics.GetGameState`)))
          (`/Game/Dynamic/CardGame/Blueprints/BP_Scoreboard.Add Points` _asbp_scoreboard _cardvalue "NewEnumerator1")
          (return _cardvalue))))))

(fn `PlayerTurnLogic`
  (returns (PlayerPoints :type Integer))
  (bind _playercardsdrawn (`self.PlayerCardsDrawn`))
  (set `self.CurrentTurn` "NewEnumerator0")
  (switch `/Game/Dynamic/CardGame/E_CurrentTurn` (`self.CurrentTurn`)
    (:`NewEnumerator0`
      (`KismetSystemLibrary.PrintString` (`KismetStringLibrary.Concat_StrStr` "Player is drawing card. Cards drawn: " (`KismetStringLibrary.Conv_IntToString` _playercardsdrawn)))
      (`/Engine/EditorBlueprintResources/StandardMacros.IncrementInt` _playercardsdrawn
        (:`  `
          (bind _carddrawn (`/Game/Dynamic/CardGame/Blueprints/BP_DeckManager.DrawCard` (`self.DeckManagerRef`)))
          (bind _output_get (set `self.PlayerCard` _carddrawn))
          (bind _returnvalue (`|SpawnActorFromClass` "/Game/Dynamic/CardGame/Blueprints/BP_Card.BP_Card_C" (`KismetMathLibrary.Conv_VectorToTransform` (`KismetMathLibrary.MakeVector` 100.0 0.0 150.0)) "Undefined" "MultiplyWithRoot" null null))
          (bind _output_get_2 (set `self.SpawnedCard` _returnvalue))
          (`/Game/Dynamic/CardGame/Blueprints/BP_Card.SetCardData` _output_get_2 (`self.PlayerCard`))
          (bind (_cardvalue _isdeathcard_) (break `/Game/Dynamic/CardGame/S_Card` _output_get))
          (if _isdeathcard_
            (`KismetSystemLibrary.PrintString` "player drew death")
            (set `self.PlayerDrewDeath` true)
            (else
              (`KismetSystemLibrary.PrintString` (`KismetStringLibrary.Conv_IntToString` _cardvalue))
              (bind _asbp_scoreboard (cast `/Game/Dynamic/CardGame/Blueprints/BP_Scoreboard` (`GameplayStatics.GetGameState`)))
              (`/Game/Dynamic/CardGame/Blueprints/BP_Scoreboard.Add Points` _asbp_scoreboard _cardvalue "NewEnumerator0")
              (return _cardvalue))))))))

(fn `UserConstructionScript`)