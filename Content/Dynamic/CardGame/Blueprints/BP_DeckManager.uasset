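; BP_DeckManager is a card-game deck manager that builds, shuffles, draws from and resets a deck of data-table cards.
; InitialiseDeck appends every CardDataTable row to Deck, and ShuffleDeck copies Deck into ShuffledDeck and randomises it.
; DrawCard removes index 0, then returns the new index 0, with debug prints throughout.
; ResetDeck clears only ShuffledDeck before re-running initialise and shuffle, so Deck accumulates duplicates on repeat calls.
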(event `self.ReceiveBeginPlay`)

(fn `DrawCard`
  (returns (CardDrawn :type "/Game/Dynamic/CardGame/CardStruct Structure"))
  (bind _output (`|GetArrayItem` (`self.ShuffledDeck`)))
  (if (> (`KismetArrayLibrary.Array_Length` (`self.ShuffledDeck`)) 0)
    (`KismetSystemLibrary.PrintString` (`KismetStringLibrary.Conv_IntToString` (`.CardValue_3_B3BF57CA4D36FB4AABCD32961A7C4028` (break `/Game/Dynamic/CardGame/CardStruct` _output))))
    (`KismetArrayLibrary.Array_Remove` (`self.ShuffledDeck`))
    (`KismetSystemLibrary.PrintString` (`KismetStringLibrary.Conv_IntToString` (`KismetArrayLibrary.Array_Length` (`self.ShuffledDeck`))))
    (return _output)
    (else
      (`KismetSystemLibrary.PrintString` "Deck Empty"))))

(fn `InitialiseDeck`
  (bind _outrownames (`DataTableFunctionLibrary.GetDataTableRowNames` (`self.CardDataTable`)))
  (for _array_element _outrownames
    (bind _returnvalue (`|GetDataTableRow` (`self.CardDataTable`) _array_element)
      (:`then`
        (`KismetArrayLibrary.Array_Add` (`self.Deck`) _returnvalue)
        (set `self.ShuffledDeck` (`|MakeArray` (struct) :!type "/Game/Dynamic/CardGame/CardStruct Structure")))))
  (for _array_element_2 (`self.Deck`)
    (`KismetSystemLibrary.PrintString` (`KismetStringLibrary.Conv_IntToString` (`.CardValue_3_B3BF57CA4D36FB4AABCD32961A7C4028` (break `/Game/Dynamic/CardGame/CardStruct` _array_element_2))))))

(fn `ResetDeck`
  (`KismetArrayLibrary.Array_Clear` (`self.ShuffledDeck`))
  (`self.InitialiseDeck`)
  (`self.ShuffleDeck`))

(fn `ShuffleDeck`
  (bind _output_get (set `self.ShuffledDeck` (`self.Deck`)))
  (`KismetArrayLibrary.Array_Shuffle` _output_get)
  (bind _output_get_2 (set `self.ShuffledDeck` (`self.ShuffledDeck`)))
  (for _array_element _output_get_2
    (`KismetSystemLibrary.PrintString` (`KismetStringLibrary.Conv_IntToString` (`.CardValue_3_B3BF57CA4D36FB4AABCD32961A7C4028` (break `/Game/Dynamic/CardGame/CardStruct` _array_element))))))

(fn `UserConstructionScript`)