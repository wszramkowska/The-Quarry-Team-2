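; BP_Scoreboard is the card game's scoreboard, recording points for the player and the AI and deciding the winner.
; AddPoints appends a value to the player or AI array according to the turn.
; CalculatePoints sums both arrays into final totals and flags the higher side's high score, with ties going to the AI.
; Results are reported only through debug Print String calls, and the totals are not reset before summing.
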(fn `Add Points`
  (params (Points :type Integer) (Turn :type "/Game/Dynamic/CardGame/E_CurrentTurn Enum" :default "NewEnumerator0"))
  (switch `/Game/Dynamic/CardGame/E_CurrentTurn` Turn
    (:`NewEnumerator0`
      ;[0 0.6134 1] Player
      (`KismetArrayLibrary.Array_Add` (`self.PlayerPoints`) Points)
      (`KismetSystemLibrary.PrintString` (`KismetStringLibrary.Concat_StrStr` "Added card number " (`KismetStringLibrary.Conv_IntToString` Points) " to PlayerPoints Array")))
    (:`NewEnumerator1`
      ;[1 0.05203 0.06197] AI
      (`KismetArrayLibrary.Array_Add` (`self.AI Points`) Points)
      (`KismetSystemLibrary.PrintString` (`KismetStringLibrary.Concat_StrStr` "Added card number " (`KismetStringLibrary.Conv_IntToString` Points) " to AIPoints Array")))))

(fn `CalculatePoints`
  (bind _playerfinalpoints (`self.PlayerFinalPoints`))
  (bind _ai_finalpoints (`self.AI FinalPoints`))
  ;[0.1475 0.502 1] Player
  (for _array_element (`self.PlayerPoints`)
    (set `self.PlayerFinalPoints` (+ (`self.PlayerFinalPoints`) _array_element)))
  ;[1 0.09351 0.1134] AI
  (for _array_element_2 (`self.AI Points`)
    (set `self.AI FinalPoints` (+ (`self.AI FinalPoints`) _array_element_2)))
  (`KismetSystemLibrary.PrintString` (`KismetStringLibrary.Concat_StrStr` "Player Points: " (`KismetStringLibrary.Conv_IntToString` _playerfinalpoints) " | AI Points:" (`KismetStringLibrary.Conv_IntToString` _ai_finalpoints)))
  (if (> _playerfinalpoints _ai_finalpoints)
    (`KismetSystemLibrary.PrintString` "Player wins!")
    (set `self.PlayerHighScore` true)
    (else
      (`KismetSystemLibrary.PrintString` "AI wins!")
      (set `self.AIHighScore` true))))

(fn `UserConstructionScript`)